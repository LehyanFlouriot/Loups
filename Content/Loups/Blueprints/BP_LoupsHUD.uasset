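; BP_LoupsHUD is the HUD for the Loups game, owning the main UI and the visibility of its roles selection panel.
; On BeginPlay it creates W_MainWidget for the first player controller, adds it to the viewport and stores the reference.
; Show and hide functions toggle the nested WRolesSelection widget between Visible and Collapsed through that stored reference.
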(event EventBeginPlay
  (bind _returnvalue (UserInterface|CreateWidget "/Game/Loups/UI/W_MainWidget.W_MainWidget_C" (Game|GetPlayerController 0)))
  (UserInterface|Viewport|AddtoViewport _returnvalue 0)
  (Variables|Default|SetMainWidget _returnvalue))

(fn ConstructionScript)

(fn ShowRolesSelectionWidget
  (Widget|SetVisibility (Variables|/Game/Loups/UI/W_MainWidget.W_MainWidget_C|GetW_RolesSelection (Variables|Default|GetMainWidget)) "Visible"))

(fn HideRolesSelectionWidget
  (Widget|SetVisibility (Variables|/Game/Loups/UI/W_MainWidget.W_MainWidget_C|GetW_RolesSelection (Variables|Default|GetMainWidget)) "Collapsed"))