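; Game mode for a Werewolf-style social deduction game, handling role selection, assignment and per-role turns.
; Role selection opens a widget on every player controller; submitted roles are stored in the game state, shuffled and dealt to player states.
; StartTurn and EndTurn activate or deactivate the matching role component on living players' characters.
; Day/night, voting, kills and role abilities are empty stubs, and lifecycle events only print debug strings.
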(event EventBeginPlay
  (Utilities|Casting|CastToBP_LoupsGameState (Game|GetGameState)))

(event EventOnRestartPlayer
  (params (NewPlayer :type Controller%20Object%20Reference))
  (Development|PrintString "On restart player"))

(event EventOnLogout
  (params (ExitingController :type Controller%20Object%20Reference))
  (Development|PrintString "On logout"))

(event EventDestroyed
  (Development|PrintString "Game mode destroyed"))

(fn ConstructionScript
  (Development|PrintString "GameMode construct"))

(fn StartRolesSelection
  (Widgets|ShowRolesSelectionWidget))

(fn AttributeRoles
  (bind _asbp_loups_game_state (Utilities|Casting|CastToBP_LoupsGameState (Game|GetGameState)))
  (Utilities|Array|Shuffle (Variables|/Game/Loups/Blueprints/BP_LoupsGameState.BP_LoupsGameState_C|GetGameRoles _asbp_loups_game_state))
  (for (_array_element _array_index) (Variables|/Script/Engine.GameStateBase|GetPlayerArray _asbp_loups_game_state)
    (bind _asbp_loups_player_state (Utilities|Casting|CastToBP_LoupsPlayerState _array_element))
    (Variables|/Game/Loups/Blueprints/BP_LoupsPlayerState.BP_LoupsPlayerState_C|SetGameRole _asbp_loups_player_state (Utilities|Array|Get(acopy) (Variables|/Game/Loups/Blueprints/BP_LoupsGameState.BP_LoupsGameState_C|GetGameRoles _asbp_loups_game_state) _array_index)))
  (GameLoop|StartGame))

(fn StartGame)

(fn SetNight)

(fn TpPlayerstoCimetery)

(fn RevivePlayer)

(fn KillPlayer)

(fn SetDay)

(fn TpPlayerstoVote)

(fn StartVote)

(fn EndVote)

(fn ActivateRole
  (params (Role :type ERole%20Enum :default "NewEnumerator0"))
  (for _array_element (Variables|/Script/Engine.GameStateBase|GetPlayerArray (Game|GetGameState))
    (bind _asbp_loups_player_state (Utilities|Casting|CastToBP_LoupsPlayerState _array_element))
    (if (Variables|/Game/Loups/Blueprints/BP_LoupsPlayerState.BP_LoupsPlayerState_C|GetIsAlive _asbp_loups_player_state)
      (if true
        (if (Utilities|Enum|Equal(Enum) (Variables|/Game/Loups/Blueprints/BP_LoupsPlayerState.BP_LoupsPlayerState_C|GetGameRole _asbp_loups_player_state) Role)
          (bind _asbp_loups_character (Utilities|Casting|CastToBP_LoupsCharacter (PlayerState|GetPawn _asbp_loups_player_state)))
          (switch Utilities|FlowControl|Switch|SwitchonERole Role
            (:NewEnumerator0
              (Components|Activation|Activate (Variables|/Game/Loups/Blueprints/BP_LoupsCharacter.BP_LoupsCharacter_C|GetTownfolkComponent _asbp_loups_character) false))
            (:NewEnumerator1
              (Components|Activation|Activate (Variables|/Game/Loups/Blueprints/BP_LoupsCharacter.BP_LoupsCharacter_C|GetFortuneTellerComponent _asbp_loups_character) false))
            (:NewEnumerator2
              (Components|Activation|Activate (Variables|/Game/Loups/Blueprints/BP_LoupsCharacter.BP_LoupsCharacter_C|GetWitchComponent _asbp_loups_character) false))
            (:NewEnumerator3
              (Components|Activation|Activate (Variables|/Game/Loups/Blueprints/BP_LoupsCharacter.BP_LoupsCharacter_C|GetWolfComponent _asbp_loups_character) false))
            (:NewEnumerator4
              (Components|Activation|Activate (Variables|/Game/Loups/Blueprints/BP_LoupsCharacter.BP_LoupsCharacter_C|GetCupidoComponent _asbp_loups_character) false))
            (:NewEnumerator5
              (Components|Activation|Activate (Variables|/Game/Loups/Blueprints/BP_LoupsCharacter.BP_LoupsCharacter_C|GetHunterComponent _asbp_loups_character) false))
            (:NewEnumerator6
              (Components|Activation|Activate (Variables|/Game/Loups/Blueprints/BP_LoupsCharacter.BP_LoupsCharacter_C|GetSherifComponent _asbp_loups_character) false))
            (:NewEnumerator7
              (Components|Activation|Activate (Variables|/Game/Loups/Blueprints/BP_LoupsCharacter.BP_LoupsCharacter_C|GetLittleGirlComponent _asbp_loups_character) false))
            (:NewEnumerator8
              (Components|Activation|Activate (Variables|/Game/Loups/Blueprints/BP_LoupsCharacter.BP_LoupsCharacter_C|GetThiefComponent _asbp_loups_character) false))))))))

(fn DeactivateRole
  (params (Role :type ERole%20Enum :default "NewEnumerator0"))
  (for _array_element (Variables|/Script/Engine.GameStateBase|GetPlayerArray (Game|GetGameState))
    (bind _asbp_loups_player_state (Utilities|Casting|CastToBP_LoupsPlayerState _array_element))
    (if (Variables|/Game/Loups/Blueprints/BP_LoupsPlayerState.BP_LoupsPlayerState_C|GetIsAlive _asbp_loups_player_state)
      (if true
        (if (Utilities|Enum|Equal(Enum) (Variables|/Game/Loups/Blueprints/BP_LoupsPlayerState.BP_LoupsPlayerState_C|GetGameRole _asbp_loups_player_state) Role)
          (bind _asbp_loups_character (Utilities|Casting|CastToBP_LoupsCharacter (PlayerState|GetPawn _asbp_loups_player_state)))
          (switch Utilities|FlowControl|Switch|SwitchonERole Role
            (:NewEnumerator0
              (Components|Activation|Deactivate (Variables|/Game/Loups/Blueprints/BP_LoupsCharacter.BP_LoupsCharacter_C|GetTownfolkComponent _asbp_loups_character)))
            (:NewEnumerator1
              (Components|Activation|Deactivate (Variables|/Game/Loups/Blueprints/BP_LoupsCharacter.BP_LoupsCharacter_C|GetFortuneTellerComponent _asbp_loups_character)))
            (:NewEnumerator2
              (Components|Activation|Deactivate (Variables|/Game/Loups/Blueprints/BP_LoupsCharacter.BP_LoupsCharacter_C|GetWitchComponent _asbp_loups_character)))
            (:NewEnumerator3
              (Components|Activation|Deactivate (Variables|/Game/Loups/Blueprints/BP_LoupsCharacter.BP_LoupsCharacter_C|GetWolfComponent _asbp_loups_character)))
            (:NewEnumerator4
              (Components|Activation|Deactivate (Variables|/Game/Loups/Blueprints/BP_LoupsCharacter.BP_LoupsCharacter_C|GetCupidoComponent _asbp_loups_character)))
            (:NewEnumerator5
              (Components|Activation|Deactivate (Variables|/Game/Loups/Blueprints/BP_LoupsCharacter.BP_LoupsCharacter_C|GetHunterComponent _asbp_loups_character)))
            (:NewEnumerator6
              (Components|Activation|Deactivate (Variables|/Game/Loups/Blueprints/BP_LoupsCharacter.BP_LoupsCharacter_C|GetSherifComponent _asbp_loups_character)))
            (:NewEnumerator7
              (Components|Activation|Deactivate (Variables|/Game/Loups/Blueprints/BP_LoupsCharacter.BP_LoupsCharacter_C|GetLittleGirlComponent _asbp_loups_character)))
            (:NewEnumerator8
              (Components|Activation|Deactivate (Variables|/Game/Loups/Blueprints/BP_LoupsCharacter.BP_LoupsCharacter_C|GetThiefComponent _asbp_loups_character)))))))))

(fn StartTurn
  (params (Role :type ERole%20Enum :default "NewEnumerator0"))
  (GameLoop|ActivateRole Role))

(fn EndTurn
  (params (Role :type ERole%20Enum :default "NewEnumerator0"))
  (GameLoop|DeactivateRole Role))

(fn Reveal
  (params (ToReveal :type BP%20Loups%20Character%20Object%20Reference%20%28by%20ref%29) (IsRevealing :type BP%20Loups%20Character%20Object%20Reference%20%28by%20ref%29)))

(fn ShootCupidoArrow
  (params (ArrowStartTransform :type Transform%20%28by%20ref%29) (Instigator :type BP%20Loups%20Character%20Object%20Reference%20%28by%20ref%29)))

(fn SetLover
  (params (Lover :type BP%20Loups%20Character%20Object%20Reference%20%28by%20ref%29)))

(fn Eat
  (params (Eaten :type BP%20Loups%20Character%20Object%20Reference%20%28by%20ref%29) (Eater :type BP%20Loups%20Character%20Object%20Reference%20%28by%20ref%29)))

(fn Charge
  (params (Charger :type BP%20Loups%20Character%20Object%20Reference%20%28by%20ref%29)))

(fn UsePotion
  (params (Instigator :type BP%20Loups%20Character%20Object%20Reference%20%28by%20ref%29) (Victim :type BP%20Loups%20Character%20Object%20Reference%20%28by%20ref%29) (Potion :type EPotion%20Enum :default "NewEnumerator0")))

(fn VoteAgainst
  (params (Voter :type BP%20Loups%20Character%20Object%20Reference%20%28by%20ref%29) (Voted :type BP%20Loups%20Character%20Object%20Reference%20%28by%20ref%29)))

(fn ShowRolesSelectionWidget
  (for _array_element (Variables|/Script/Engine.GameStateBase|GetPlayerArray (Game|GetGameState))
    (bind _asbp_loups_player_controller (Utilities|Casting|CastToBP_LoupsPlayerController (Game|GetPlayerController _array_element)))
    (Default|ServerShowRolesSelectionWidget _asbp_loups_player_controller)))

(fn SubmitRolesSelection
  (params (Roles :type Array%20of%20ERole%20Enums :default "NewEnumerator9"))
  (bind _asbp_loups_game_state (Utilities|Casting|CastToBP_LoupsGameState (Game|GetGameState)))
  (Variables|/Game/Loups/Blueprints/BP_LoupsGameState.BP_LoupsGameState_C|SetGameRoles _asbp_loups_game_state Roles)
  (GameLoop|AttributeRoles))