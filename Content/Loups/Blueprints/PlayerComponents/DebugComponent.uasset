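; Debug actor component for Loups characters that shows each player's game role in the world.
; Every tick it reads GameRole from the owning BP_LoupCharacter's BP_LoupsPlayerState and draws it as debug text above the actor.
; Two further helpers, currently not called, print the game state's PlayState and draw a green or red sphere by whether the character is locally controlled.
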(event EventTick
  (params (DeltaSeconds :type Float%20%28single-precision%29))
  (CallFunction|DebugRole))

(fn DebugRole
  (bind _returnvalue (Components|GetOwner))
  (bind _asbp_loup_character (Utilities|Casting|CastToBP_LoupCharacter _returnvalue))
  (bind _asbp_loups_player_state (Utilities|Casting|CastToBP_LoupsPlayerState (Variables|/Script/Engine.Pawn|GetPlayerState _asbp_loup_character)))
  (Rendering|Debug|DrawDebugString (+ (Transformation|GetActorLocation _returnvalue) "0.000000,0.000000,100.000000") (Utilities|String|EnumtoString (Variables|/Game/Loups/Blueprints/BP_LoupsPlayerState.BP_LoupsPlayerState_C|GetGameRole _asbp_loups_player_state)) 0 "(R=1.000000,G=1.000000,B=1.000000,A=1.000000)"))

(fn DebugGameState
  (bind _asbp_loups_game_state (Utilities|Casting|CastToBP_LoupsGameState (Game|GetGameState)))
  (Development|PrintString (Utilities|String|EnumtoString (Variables|/Game/Loups/Blueprints/BP_LoupsGameState.BP_LoupsGameState_C|GetPlayState _asbp_loups_game_state)) true false "(R=0.000000,G=0.660000,B=1.000000,A=1.000000)" 0.0 "PlayState"))

(fn DebugLocallyControlled
  (bind _returnvalue (Components|GetOwner))
  (bind _returnvalue_2 (Transformation|GetActorLocation _returnvalue))
  (bind _returnvalue_3 (+ _returnvalue_2 ""))
  (bind _asbp_loup_character (Utilities|Casting|CastToBP_LoupCharacter (Components|GetOwner)))
  (if (Pawn|IsLocallyControlled _asbp_loup_character)
    (Rendering|Debug|DrawDebugSphere _returnvalue_3 1e+02 12 "(R=0.000000,G=1.000000,B=0.084394,A=1.000000)" 0.0)
    (else
      (Rendering|Debug|DrawDebugSphere _returnvalue_3 1e+02 12 "(R=1.000000,G=0.000000,B=0.042518,A=1.000000)" 0.0))))