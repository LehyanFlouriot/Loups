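; NameComponent is a component that shows the owning character's player name above it in the Loups game.
; Every tick it checks the GameTime value on BP_LoupsGameState and continues only during the enum's first listed state.
; It then reads the name from the character's BP_LoupsPlayerState and draws it with DrawDebugString just above the actor's location, using debug text rather than a widget.
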(event EventTick
  (params (DeltaSeconds :type Float%20%28single-precision%29))
  (bind _asbp_loups_game_state (Utilities|Casting|CastToBP_LoupsGameState (Game|GetGameState)))
  (if (Utilities|Enum|Equal(Enum) (Variables|/Game/Loups/Blueprints/BP_LoupsGameState.BP_LoupsGameState_C|GetGameTime _asbp_loups_game_state) "NewEnumerator0")
    (bind _ascharacter (Utilities|Casting|CastToCharacter (Components|GetOwner)))
    (bind _asbp_loups_player_state (Utilities|Casting|CastToBP_LoupsPlayerState (Variables|/Script/Engine.Pawn|GetPlayerState _ascharacter)))
    (Rendering|Debug|DrawDebugString (+ (Transformation|GetActorLocation _ascharacter) "0.000000,0.000000,100.000000") (PlayerState|GetPlayerName _asbp_loups_player_state) 0 "(R=1.000000,G=1.000000,B=1.000000,A=1.000000)")))