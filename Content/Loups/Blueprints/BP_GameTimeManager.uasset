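; BP_GameTimeManager fades a scene light between day and night according to the game time held in BP_LoupsGameState.
; Every tick it reads GameTime and interpolates the light's intensity with FInterpTo, brightening it in Jour and dimming it to zero in Nuit.
; The fade to night runs at a much higher interpolation speed than the very gradual return to daylight.
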(event EventTick
  (params (DeltaSeconds :type Float%20%28single-precision%29))
  (bind _light (Variables|Default|GetLight))
  (bind _lightcomponent (Variables|/Script/Engine.Light|GetLightComponent _light))
  (bind _intensity (Variables|/Script/Engine.LightComponentBase|GetIntensity _lightcomponent))
  (bind _asbp_loups_game_state (Utilities|Casting|CastToBP_LoupsGameState (Game|GetGameState)))
  (switch Utilities|FlowControl|Switch|SwitchonEGameTime (Variables|/Game/Loups/Blueprints/BP_LoupsGameState.BP_LoupsGameState_C|GetGameTime _asbp_loups_game_state)
    (:NewEnumerator0
      (Rendering|Components|Light|SetIntensity _lightcomponent (Math|Interpolation|FInterpTo _intensity 3.0 DeltaSeconds 0.01)))
    (:NewEnumerator1
      (Rendering|Components|Light|SetIntensity _lightcomponent (Math|Interpolation|FInterpTo _intensity 0.0 DeltaSeconds 1.0)))))

(fn ConstructionScript)